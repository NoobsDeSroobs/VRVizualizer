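; Right-hand Vive motion controller actor that maps VR input to menu, grab and teleport actions.
; Shoulder toggles the child-actor BP_Menu, thumbstick X also pitches it, trigger drives the Grabber, and face buttons call ToggleCP or launch a TeleportationBubble along controller forward.
; Tick forwards cached thumbstick axes to the ViveController child actor as touch position.
; Older highlight and attach-based holding logic remains disconnected, and overlap events are empty.
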(event Collision|EventActorBeginOverlap
  (params (OtherActor :type Actor%20Object%20Reference))
  ;[1 1 1] Handle overalp
)

(event EventBeginPlay
  (Input|EnableInput (Game|GetPlayerController 0))
  (Actor|Tick|SetActorTickEnabled true))

(event Collision|EventActorEndOverlap
  (params (OtherActor :type Actor%20Object%20Reference))
  ;[1 1 1] Handle overalp
)

(event EventTick
  (params (DeltaSeconds :type Float%20%28single-precision%29))
  (bind _asvive_controller (Utilities|Casting|CastToViveController (Variables|/Script/Engine.ChildActorComponent|GetChildActor (Variables|Default|GetControllerBP))))
  (Default|UpdateTouchPos _asvive_controller (Variables|Default|GetTouchX) (Variables|Default|GetTouchY)))

(event Input|KeyboardEvents|MotionControllerRightThumbstickX
  (params (AxisValue :type Float%20%28single-precision%29))
  ;[1 1 1] Rotation of menu
  (Transformation|AddActorLocalRotation (Variables|/Script/Engine.ChildActorComponent|GetChildActor (Variables|Default|GetBP_Menu)) (Math|Rotator|MakeRotator 0.0 AxisValue 0.0) false false))

(event Input|KeyboardEvents|MotionControllerRightThumbstickY
  (params (AxisValue :type Float%20%28single-precision%29))
  (Variables|Default|SetTouchY AxisValue))

(event Input|KeyboardEvents|MotionControllerRightThumbstickX
  (params (AxisValue :type Float%20%28single-precision%29))
  (Variables|Default|SetTouchX AxisValue))

(event Input|KeyboardEvents|MotionControllerRightTrigger
  (params (Key :type Key%20Structure :default "AnyKey"))
  (bind _grabber (Variables|Default|GetGrabber))
  ;[1 1 1] Grab Actors
  (:Pressed
    (Class|GrabberComponent|GrabOverlappingActor _grabber))
  (:Released
    (Class|GrabberComponent|ReleaseOverlappingActor _grabber)))

(event Input|KeyboardEvents|MotionControllerRightShoulder
  (params (Key :type Key%20Structure :default "AnyKey"))
  ;[1 1 1] Toggle the ingame menu HUD
  (:Pressed
    (bind _asbp_menu (Utilities|Casting|CastToBP_Menu (Variables|/Script/Engine.ChildActorComponent|GetChildActor (Variables|Default|GetBP_Menu)))
      (:then
        (Default|ToggleMenu _asbp_menu))
      (:CastFailed
        (Development|PrintString "Failed cast to menu")))))

(event Input|KeyboardEvents|MotionControllerRightFaceButton1
  (params (Key :type Key%20Structure :default "AnyKey"))
  (bind _controllerbp (Variables|Default|GetControllerBP))
  (bind _returnvalue (Transformation|GetWorldTransform _controllerbp))
  (bind (_location _rotation _scale) (Math|Transform|BreakTransform _returnvalue))
  ;[1 1 1] Handle teleportation
  (:Released
    (bind _returnvalue_2 (Game|SpawnActorfromClass "/Game/Teleporter/TeleportationBubble.TeleportationBubble_C" (Math|Transform|MakeTransform (+ _location (* (Math|Vector|GetForwardVector _controllerbp) 1e+01)) _rotation _scale) "AlwaysSpawn" self 0))
    (Default|Fly _returnvalue_2 (* (Math|Vector|GetForwardVector (Variables|Default|GetControllerBP)) (Variables|Default|GetProjectileSpeed)))))

(event Input|KeyboardEvents|MotionControllerRightFaceButton3
  (params (Key :type Key%20Structure :default "AnyKey"))
  (:Released
    (Default|CallToggleCP)))

(fn ConstructionScript
  (Variables|Default|SetProjectileSpeed 5e+04))