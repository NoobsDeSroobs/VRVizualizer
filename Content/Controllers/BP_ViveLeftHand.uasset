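; Left-hand Vive motion controller that grabs actors, toggles a level selector menu and shows readouts on a text render.
; Input feeds the child controller's visuals and the Grabber, whose overlaps receive previous/next calls through PlaybackControlls; play/pause is unwired.
; While face button 1 is held, a Tick-driven gate shows model-scaled distance between both pointers.
; A line trace subscribes to a DataSetBP, whose counter then overwrites the text each tick.
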(event Custom|UpdateCtrlDistance
  (Utilities|FlowControl|Gate true
    (:Exit
      (Rendering|Components|TextRender|SetText (Variables|Default|GetTextRender) (Utilities|Text|ToText(Float) (/ (Math|Vector|VectorLength (- (Transformation|GetWorldLocation (Variables|/Game/Controllers/BP_ViveController.BP_ViveController_C|GetPointer (.AsBP%20Vive%20Controller (Utilities|Casting|CastToBP_ViveController (Variables|/Script/Engine.ChildActorComponent|GetChildActor (Variables|/Game/Controllers/BP_ViveRightHand.BP_ViveRightHand_C|GetControllerBP (Variables|Default|GetOtherController))))))) (Transformation|GetWorldLocation (Variables|/Game/Controllers/BP_ViveController.BP_ViveController_C|GetPointer (.AsBP%20Vive%20Controller (Utilities|Casting|CastToBP_ViveController (Variables|/Script/Engine.ChildActorComponent|GetChildActor (Variables|Default|GetControllerBP)))))))) (Variables|Default|GetScaleOfModel)) "HalfToEven" true 1 324 3)))))

(event EventBeginPlay
  (Input|EnableInput (Game|GetPlayerController 0))
  (bind _asbp_vive_controller (Utilities|Casting|CastToBP_ViveController (Variables|/Script/Engine.ChildActorComponent|GetChildActor (Variables|Default|GetControllerBP))))
  (Default|SetMaterial _asbp_vive_controller "/Game/Controllers/Parts/ViveLeftController.ViveLeftController"))

(event EventTick
  (params (DeltaSeconds :type Float%20%28single-precision%29))
  (bind _volumetodisplay (Variables|Default|GetVolumeToDisplay))
  (CallFunction|UpdateCtrlDistance)
  (bind _asbp_vive_controller (Utilities|Casting|CastToBP_ViveController (Variables|/Script/Engine.ChildActorComponent|GetChildActor (Variables|Default|GetControllerBP))))
  (Default|UpdateTouchPos _asbp_vive_controller (Variables|Default|GetTouchX) (Variables|Default|GetTouchY))
  (if (!= _volumetodisplay 0)
    (Rendering|Components|TextRender|SetText (Variables|Default|GetTextRender) (Variables|/Script/Engine.TextRenderComponent|GetText (Variables|/Game/Blueprints/DataSetBP.DataSetBP_C|GetCounter _volumetodisplay)))))

(event Input|KeyboardEvents|MotionControllerLeftThumbstickX
  (params (AxisValue :type Float%20%28single-precision%29))
  (Variables|Default|SetTouchX AxisValue))

(event Input|KeyboardEvents|MotionControllerLeftThumbstickY
  (params (AxisValue :type Float%20%28single-precision%29))
  (Variables|Default|SetTouchY AxisValue))

(event Input|KeyboardEvents|MotionControllerLeftTriggerAxis
  (params (AxisValue :type Float%20%28single-precision%29))
  (Default|UpdateTriggerPos (.AsBP%20Vive%20Controller (Utilities|Casting|CastToBP_ViveController (Variables|/Script/Engine.ChildActorComponent|GetChildActor (Variables|Default|GetControllerBP)))) AxisValue))

(event Input|KeyboardEvents|MotionControllerLeftFaceButton4
  (params (Key :type Key%20Structure :default "AnyKey"))
  (:Pressed
    (bind _asbp_vive_controller (Utilities|Casting|CastToBP_ViveController (Variables|/Script/Engine.ChildActorComponent|GetChildActor (Variables|Default|GetControllerBP))))
    (bind _returnvalue (Class|GrabberComponent|GetOverlappingActors (Variables|Default|GetGrabber) (Variables|/Script/Engine.ChildActorComponent|GetChildActor (Variables|/Game/Controllers/BP_ViveController.BP_ViveController_C|GetPointer _asbp_vive_controller))))
    (bind _array_element (Utilities|Array|ForEachLoopwithBreak _returnvalue :!label _label)
      (:LoopBody
        (if (Utilities|DoesObjectImplementInterface _array_element "/Game/Controllers/PlaybackControlls.PlaybackControlls_C")
          (Class|PlaybackControlls|Previous(Message) _array_element)
          (goto _label Break))))))

(event Input|KeyboardEvents|MotionControllerLeftFaceButton2
  (params (Key :type Key%20Structure :default "AnyKey"))
  (:Pressed
    (bind _asbp_vive_controller (Utilities|Casting|CastToBP_ViveController (Variables|/Script/Engine.ChildActorComponent|GetChildActor (Variables|Default|GetControllerBP))))
    (bind _returnvalue (Class|GrabberComponent|GetOverlappingActors (Variables|Default|GetGrabber) (Variables|/Script/Engine.ChildActorComponent|GetChildActor (Variables|/Game/Controllers/BP_ViveController.BP_ViveController_C|GetPointer _asbp_vive_controller))))
    (bind _array_element (Utilities|Array|ForEachLoopwithBreak _returnvalue :!label _label)
      (:LoopBody
        (if (Utilities|DoesObjectImplementInterface _array_element "/Game/Controllers/PlaybackControlls.PlaybackControlls_C")
          (Class|PlaybackControlls|Next(Message) _array_element)
          (goto _label Break))))))

(event Input|KeyboardEvents|MotionControllerLeftShoulder
  (params (Key :type Key%20Structure :default "AnyKey"))
  (bind _returnvalue (Transformation|GetActorLocation))
  (bind _returnvalue_2 (Transformation|GetActorRotation))
  (bind _returnvalue_3 (Math|Vector|GetForwardVector _returnvalue_2))
  (bind _returnvalue_4 (* _returnvalue_3 500))
  (bind _returnvalue_5 (+ _returnvalue _returnvalue_4))
  (bind (_x _y) (Math|Vector|BreakVector _returnvalue_5))
  (:Pressed
    (bind _asvr_pawn (Utilities|Casting|CastToVR_Pawn (Game|Player|GetPlayerPawn 0)))
    (if (== (Variables|/Game/Blueprints/VR_Pawn.VR_Pawn_C|GetMenu _asvr_pawn) 0)
      (bind _returnvalue_6 (Game|SpawnActorfromClass "/Game/3DMenus/LevelSelector.LevelSelector_C" (Math|Conversions|ToTransform(Vector) (Math|Vector|MakeVector _x _y 0.0)) "AlwaysSpawn" 0 0))
      (bind _asvr_pawn_2 (Utilities|Casting|CastToVR_Pawn (Game|Player|GetPlayerPawn 0)))
      (Variables|/Game/Blueprints/VR_Pawn.VR_Pawn_C|SetMenu _asvr_pawn_2 _returnvalue_6)
      (else
        (bind _asvr_pawn_3 (Utilities|Casting|CastToVR_Pawn (Game|Player|GetPlayerPawn 0)))
        (Actor|DestroyActor (Variables|/Game/Blueprints/VR_Pawn.VR_Pawn_C|GetMenu _asvr_pawn_3))
        (Variables|/Game/Blueprints/VR_Pawn.VR_Pawn_C|SetMenu _asvr_pawn_3 0)))))

(event Input|KeyboardEvents|MotionControllerLeftTrigger
  (params (Key :type Key%20Structure :default "AnyKey"))
  (bind _grabber (Variables|Default|GetGrabber))
  ;[1 1 1] Grab Actors
  (:Pressed
    (bind _asbp_vive_controller (Utilities|Casting|CastToBP_ViveController (Variables|/Script/Engine.ChildActorComponent|GetChildActor (Variables|Default|GetControllerBP))))
    (Class|GrabberComponent|GrabOverlappingActor _grabber (Variables|/Script/Engine.ChildActorComponent|GetChildActor (Variables|/Game/Controllers/BP_ViveController.BP_ViveController_C|GetPointer _asbp_vive_controller))))
  (:Released
    (Class|GrabberComponent|ReleaseOverlappingActor _grabber)))

(event Input|KeyboardEvents|MotionControllerLeftShoulder
  (params (Key :type Key%20Structure :default "AnyKey"))
  (bind _controllerbp (Variables|Default|GetControllerBP))
  (bind _childactor (Variables|/Script/Engine.ChildActorComponent|GetChildActor _controllerbp))
  (:Pressed
    (bind _asbp_vive_controller (Utilities|Casting|CastToBP_ViveController _childactor))
    (Default|ClickMenu _asbp_vive_controller true))
  (:Released
    (bind _asbp_vive_controller_2 (Utilities|Casting|CastToBP_ViveController _childactor))
    (Default|ClickMenu _asbp_vive_controller_2 false)))

(event Input|KeyboardEvents|MotionControllerLeftFaceButton3
  (params (Key :type Key%20Structure :default "AnyKey"))
  (:Pressed
    (CallFunction|SubscribetoVolume)))

(event Input|KeyboardEvents|MotionControllerLeftFaceButton1
  (params (Key :type Key%20Structure :default "AnyKey"))
  (:Pressed
    (Utilities|FlowControl|Gate true) ; enters at Open
  )
  (:Released
    (Utilities|FlowControl|Gate true) ; enters at Close
  ))

(fn ConstructionScript)

(fn SubscribetoVolume
  (bind _lineofsight (Variables|Default|GetLineOfSight))
  (bind _returnvalue (Transformation|GetWorldLocation _lineofsight))
  (bind _outhit (Collision|LineTraceForObjects _returnvalue (+ _returnvalue (* (Math|Vector|GetForwardVector _lineofsight) 1000)) (Utilities|Array|MakeArray "ObjectTypeQuery1") false 0 "ForOneFrame"))
  (if (Utilities|ClassIsChildOf (Utilities|GetClass (.HitActor (Collision|BreakHitResult _outhit))) "/Game/Blueprints/DataSetBP.DataSetBP_C")
    (Variables|Default|SetVolumeToDisplay (.AsData%20Set%20BP (Utilities|Casting|CastToDataSetBP (.HitActor (Collision|BreakHitResult _outhit)))))))