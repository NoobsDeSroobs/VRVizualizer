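; BP_CuttingPLane is a cutting plane actor for VR that can be switched on and off through its Toggle function.
; Activating it shows the actor, enables its collision and teleports it to the VR_Pawn's right controller transform, while deactivating hides it and disables collision.
; Toggle also sets the UseCuttingPLane scalar in a Material Parameter Collection, exposing the on/off state to materials.
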(fn ConstructionScript)

(fn Toggle
  (params (Active :type Boolean))
  (if Active
    (Rendering|SetActorHiddenInGame false)
    (Collision|SetActorEnableCollision true)
    (bind _asvr_pawn (Utilities|Casting|CastToVR_Pawn (Game|Player|GetPlayerPawn 0)))
    (bind _rightcontroller (Default|GetRightController _asvr_pawn))
    (Transformation|SetActorTransform (Transformation|GetActorTransform _rightcontroller) false true)
    (Rendering|Material|SetScalarParameterValue "/Game/MaterialParameterCollection.MaterialParameterCollection" "UseCuttingPLane" 1.0 :!class /Script/Engine.KismetMaterialLibrary)
    (else
      (Rendering|SetActorHiddenInGame true)
      (Collision|SetActorEnableCollision false)
      (Rendering|Material|SetScalarParameterValue "/Game/MaterialParameterCollection.MaterialParameterCollection" "UseCuttingPLane" 0.0 :!class /Script/Engine.KismetMaterialLibrary))))