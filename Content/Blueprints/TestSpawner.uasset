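; TestSpawner is a test actor that attaches a particle effect to its Cube component when play begins.
; BeginPlay enables ticking and spawns TestParticleSystem snapped to the Cube, with auto-destroy turned off.
; Tick accumulates a Time counter and subtracts one second whenever it reaches one, triggering nothing else.
; The overlap event and construction script are empty.
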(event EventBeginPlay
  (Actor|Tick|SetActorTickEnabled true)
  (Effects|SpawnEmitterAttached "/Game/TestParticleSystem.TestParticleSystem" (Variables|Default|GetCube) "None" "0, 0, 0" "0, 0, 0" "SnapToTarget" false) ; Spawn a boost effect on the existing engine emitters
)

(event Collision|EventActorBeginOverlap
  (params (OtherActor :type Actor%20Object%20Reference)))

(event EventTick
  (params (DeltaSeconds :type Float%20%28single-precision%29))
  (bind _output_get (Variables|Default|SetTime (+ DeltaSeconds (Variables|Default|GetTime))))
  (if (not (< _output_get 1.0))
    (Variables|Default|SetTime (- (Variables|Default|GetTime) 1.0))))

(fn ConstructionScript)