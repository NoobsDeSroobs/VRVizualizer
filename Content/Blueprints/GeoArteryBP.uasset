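; GeoArteryBP plays a looping flipbook animation of an artery by swapping eighteen static meshes on one component with a vertex colour material.
; BeginPlay divides LoopTime into per-frame SwitchTime, which Tick uses to advance frames through a gate.
; Overlaps on Play toggle the gate, while Prev and Next adjust the index.
; UpdateMesh always increments first, so Next skips a frame and Prev's decrement is cancelled.
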(event Custom|Increment
  ;[1 1 1] Increment
  (bind _result (Math|Integer|IncrementInt (Variables|Default|GetCurrentInt))
    (:%20%20
      (Variables|Default|SetCurrentInt (Math|Integer|%(Integer) _result (Utilities|Array|Length (Variables|Default|GetArteryMeshes)))))))

(event Custom|PrevBeginOverlap
  (params (OverlappedComponent :type Primitive%20Component%20Object%20Reference) (OtherActor :type Actor%20Object%20Reference) (OtherComp :type Primitive%20Component%20Object%20Reference) (OtherBodyIndex :type Integer) (bFromSweep :type Boolean) (SweepResult :type Hit%20Result%20Structure%20%28by%20ref%29))
  ;[1 1 1] Init
  (CallFunction|Decrement)
  (CallFunction|UpdateMesh))

(event Custom|PLayBeginOverlap
  (params (OverlappedComponent :type Primitive%20Component%20Object%20Reference) (OtherActor :type Actor%20Object%20Reference) (OtherComp :type Primitive%20Component%20Object%20Reference) (OtherBodyIndex :type Integer) (bFromSweep :type Boolean) (SweepResult :type Hit%20Result%20Structure%20%28by%20ref%29))
  ;[1 1 1] Init
  (Utilities|FlowControl|Gate true) ; enters at Toggle
)

(event Custom|NextBeginOverlap
  (params (OverlappedComponent :type Primitive%20Component%20Object%20Reference) (OtherActor :type Actor%20Object%20Reference) (OtherComp :type Primitive%20Component%20Object%20Reference) (OtherBodyIndex :type Integer) (bFromSweep :type Boolean) (SweepResult :type Hit%20Result%20Structure%20%28by%20ref%29))
  ;[1 1 1] Init
  (CallFunction|Increment)
  (CallFunction|UpdateMesh))

(event Custom|UpdateMesh
  ;[1 1 1] UpdateMesh
  (CallFunction|Increment)
  (Components|StaticMesh|SetStaticMesh (Variables|Default|GetArtery) (Utilities|Array|Get(acopy) (Variables|Default|GetArteryMeshes) (Variables|Default|GetCurrentInt)))
  (Rendering|Material|SetMaterial (Variables|Default|GetArtery) 0 "/Game/Materials/VertexColour.VertexColour"))

(event Custom|Decrement
  ;[1 1 1] Decrement
  (bind _result (Math|Integer|DecrementInt (Variables|Default|GetCurrentInt))
    (:%20%20
      (if (> 0 _result)
        (Variables|Default|SetCurrentInt (- (Variables|Default|GetCurrentInt) (Utilities|Array|Length (Variables|Default|GetArteryMeshes))))))))

(event EventBeginPlay
  (bind _arterymeshes (Variables|Default|GetArteryMeshes))
  (bind _arterymeshes_2 (Variables|Default|GetArteryMeshes))
  (bind _arterymeshes_3 (Variables|Default|GetArteryMeshes))
  (bind _arterymeshes_4 (Variables|Default|GetArteryMeshes))
  (bind _arterymeshes_5 (Variables|Default|GetArteryMeshes))
  ;[1 1 1] Init
  (Utilities|Array|Add _arterymeshes_2 "/Game/StaticMeshes/GeometricMeshes/ArteryGeo0.ArteryGeo0")
  (Utilities|Array|Add _arterymeshes_2 "/Game/StaticMeshes/GeometricMeshes/ArteryGeo1.ArteryGeo1")
  (Utilities|Array|Add _arterymeshes_2 "/Game/StaticMeshes/GeometricMeshes/ArteryGeo2.ArteryGeo2")
  (Utilities|Array|Add _arterymeshes_2 "/Game/StaticMeshes/GeometricMeshes/ArteryGeo3.ArteryGeo3")
  (Utilities|Array|Add _arterymeshes_3 "/Game/StaticMeshes/GeometricMeshes/ArteryGeo4.ArteryGeo4")
  (Utilities|Array|Add _arterymeshes_3 "/Game/StaticMeshes/GeometricMeshes/ArteryGeo5.ArteryGeo5")
  (Utilities|Array|Add _arterymeshes_3 "/Game/StaticMeshes/GeometricMeshes/ArteryGeo6.ArteryGeo6")
  (Utilities|Array|Add _arterymeshes_3 "/Game/StaticMeshes/GeometricMeshes/ArteryGeo7.ArteryGeo7")
  (Utilities|Array|Add _arterymeshes "/Game/StaticMeshes/GeometricMeshes/ArteryGeo8.ArteryGeo8")
  (Utilities|Array|Add _arterymeshes "/Game/StaticMeshes/GeometricMeshes/ArteryGeo9.ArteryGeo9")
  (Utilities|Array|Add _arterymeshes "/Game/StaticMeshes/GeometricMeshes/ArteryGeo10.ArteryGeo10")
  (Utilities|Array|Add _arterymeshes "/Game/StaticMeshes/GeometricMeshes/ArteryGeo11.ArteryGeo11")
  (Utilities|Array|Add _arterymeshes_4 "/Game/StaticMeshes/GeometricMeshes/ArteryGeo12.ArteryGeo12")
  (Utilities|Array|Add _arterymeshes_4 "/Game/StaticMeshes/GeometricMeshes/ArteryGeo13.ArteryGeo13")
  (Utilities|Array|Add _arterymeshes_4 "/Game/StaticMeshes/GeometricMeshes/ArteryGeo14.ArteryGeo14")
  (Utilities|Array|Add _arterymeshes_4 "/Game/StaticMeshes/GeometricMeshes/ArteryGeo15.ArteryGeo15")
  (Utilities|Array|Add _arterymeshes_5 "/Game/StaticMeshes/GeometricMeshes/ArteryGeo16.ArteryGeo16")
  (Utilities|Array|Add _arterymeshes_5 "/Game/StaticMeshes/GeometricMeshes/ArteryGeo17.ArteryGeo17")
  (Variables|Default|SetSwitchTime (/ (Variables|Default|GetLoopTime) (Math|Conversions|ToFloat(Integer) (Utilities|Array|Length (Variables|Default|GetArteryMeshes)))))
  (Collision|AssignOnComponentBeginOverlap (Variables|Default|GetPrev) (delegate Custom|PrevBeginOverlap))
  (Collision|AssignOnComponentBeginOverlap (Variables|Default|GetPlay) (delegate Custom|PLayBeginOverlap))
  (Collision|AssignOnComponentBeginOverlap (Variables|Default|GetNext) (delegate Custom|NextBeginOverlap)))

(event EventTick
  (params (DeltaSeconds :type Float%20%28single-precision%29))
  (Utilities|FlowControl|Gate true
    (:Exit
      (bind _output_get (Variables|Default|SetCurrentTime (+ DeltaSeconds (Variables|Default|GetCurrentTime))))
      (if (> _output_get (Variables|Default|GetSwitchTime))
        (Variables|Default|SetCurrentTime (- (Variables|Default|GetCurrentTime) (Variables|Default|GetSwitchTime)))
        (CallFunction|UpdateMesh)))))

(fn ConstructionScript)