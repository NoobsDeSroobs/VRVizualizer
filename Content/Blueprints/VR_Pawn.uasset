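; VR player pawn that carries a camera and a Vive right-hand controller as a child actor, and supports teleporting.
; GetRightController returns that child actor cast to BP_ViveRightHand.
; Teleport moves the pawn to a target location with no sweep, ignoring a near-zero target.
; A horizontal camera-offset correction for the target is present but unused, so the pawn origin lands on the target.
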(fn ConstructionScript)

(fn GetRightController
  (bind _asbp_vive_right_hand (Utilities|Casting|CastToBP_ViveRightHand (Variables|/Script/Engine.ChildActorComponent|GetChildActor (Variables|Default|GetBP_ViveRightHand))))
  (return _asbp_vive_right_hand))

(fn Teleport
  (params (TargetLocation :type Vector))
  (if (Math|Vector|NotEqual(Vector) TargetLocation "0, 0, 0" 0.0001)
    (Transformation|SetActorLocation TargetLocation false true)))