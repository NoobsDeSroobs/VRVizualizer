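; Volume actor that displays a sequence of 3D artery datasets, or a single supplied texture, through a volume material.
; BeginPlay fills the texture array; Tick calls UpdateData, zeroes rotation, advances the frame and updates the counter text.
; UpdateMaterial creates a new dynamic material instance on every call, passing it the current texture, slice size, threshold and Min/Max component bounds.
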(event Custom|UpdateMaterial
  (bind _returnvalue (Rendering|Material|CreateDynamicMaterialInstance "/Game/Materials/ArteryMats/TestVolumeBaseMaterial.TestVolumeBaseMaterial" :!class /Script/Engine.KismetMaterialLibrary))
  (Rendering|Material|SetTextureParameterValue _returnvalue "VolumeTexture" (Utilities|Array|Get(acopy) (Variables|Default|GetTextures) (Variables|Default|GetCurrentIndex)))
  (Rendering|Material|SetScalarParameterValue _returnvalue "TextureXSize" (Variables|Default|GetTexSliceWidth) :!class /Script/Engine.MaterialInstanceDynamic)
  (Rendering|Material|SetScalarParameterValue _returnvalue "TextureYSize" (Variables|Default|GetTex%20Slice%20Height) :!class /Script/Engine.MaterialInstanceDynamic)
  (Rendering|Material|SetVectorParameterValue _returnvalue "Bounding Min" (Math|Conversions|ToLinearColor(Vector) (Transformation|GetWorldLocation (Variables|Default|Getmin))) :!class /Script/Engine.MaterialInstanceDynamic)
  (Rendering|Material|SetVectorParameterValue _returnvalue "Bounding Max" (Math|Conversions|ToLinearColor(Vector) (Transformation|GetWorldLocation (Variables|Default|Getmax))) :!class /Script/Engine.MaterialInstanceDynamic)
  (Rendering|Material|SetScalarParameterValue _returnvalue "Intensity Threshold" (Variables|Default|GetThreshold) :!class /Script/Engine.MaterialInstanceDynamic)
  (Rendering|Material|SetMaterial (Variables|Default|GetVolume) 0 _returnvalue))

(event Custom|IncrementTexID
  (Variables|Default|SetCurrentIndex (Utilities|Increment (Variables|Default|GetCurrentIndex) (Variables|Default|GetTextures)))
  (CallFunction|UpdateMaterial))

(event EventBeginPlay
  (bind _texture (Variables|Default|GetTexture))
  (if (!= _texture 0)
    (Utilities|Array|Add (Variables|Default|GetTextures) _texture)
    (else
      (Utilities|Array|Add (Variables|Default|GetTextures) "/Game/Materials/ArteryMats/ArteryAnim/artery0_0.artery0_0")
      (Utilities|Array|Add (Variables|Default|GetTextures) "/Game/Materials/ArteryMats/ArteryAnim/artery1_0.artery1_0")
      (Utilities|Array|Add (Variables|Default|GetTextures) "/Game/Materials/ArteryMats/ArteryAnim/artery2_0.artery2_0")
      (Utilities|Array|Add (Variables|Default|GetTextures) "/Game/Materials/ArteryMats/ArteryAnim/artery3_0.artery3_0")
      (Utilities|Array|Add (Variables|Default|GetTextures) "/Game/Materials/ArteryMats/ArteryAnim/artery4_0.artery4_0")
      (Utilities|Array|Add (Variables|Default|GetTextures) "/Game/Materials/ArteryMats/ArteryAnim/artery5_0.artery5_0")
      (Utilities|Array|Add (Variables|Default|GetTextures) "/Game/Materials/ArteryMats/ArteryAnim/artery6_0.artery6_0")
      (Utilities|Array|Add (Variables|Default|GetTextures) "/Game/Materials/ArteryMats/ArteryAnim/artery7_0.artery7_0")
      (Utilities|Array|Add (Variables|Default|GetTextures) "/Game/Materials/ArteryMats/ArteryAnim/artery8_0.artery8_0")
      (Utilities|Array|Add (Variables|Default|GetTextures) "/Game/Materials/ArteryMats/ArteryAnim/artery9_0.artery9_0")
      (Utilities|Array|Add (Variables|Default|GetTextures) "/Game/Materials/ArteryMats/ArteryAnim/artery10_0.artery10_0")
      (Utilities|Array|Add (Variables|Default|GetTextures) "/Game/Materials/ArteryMats/ArteryAnim/artery11_0.artery11_0")
      (Utilities|Array|Add (Variables|Default|GetTextures) "/Game/Materials/ArteryMats/ArteryAnim/artery12_0.artery12_0")
      (Utilities|Array|Add (Variables|Default|GetTextures) "/Game/Materials/ArteryMats/ArteryAnim/artery13_0.artery13_0")
      (Utilities|Array|Add (Variables|Default|GetTextures) "/Game/Materials/ArteryMats/ArteryAnim/artery14_0.artery14_0")
      (Utilities|Array|Add (Variables|Default|GetTextures) "/Game/Materials/ArteryMats/ArteryAnim/artery15_0.artery15_0")
      (Utilities|Array|Add (Variables|Default|GetTextures) "/Game/Materials/ArteryMats/ArteryAnim/artery17_0.artery17_0")
      (CallFunction|UpdateMaterial))))

(event EventTick
  (params (DeltaSeconds :type Float%20%28single-precision%29))
  (bind _textures (Variables|Default|GetTextures))
  (bind _returnvalue (Utilities|Array|Length _textures))
  (|CallParentFunction DeltaSeconds)
  (Class|Grabbable|UpdateData)
  (Transformation|SetActorRotation "0, 0, 0")
  (CallFunction|IncrementTexID) ; Limit the following code by a timed gate.
  (CallFunction|UpdateMaterial)
  (bind _stringnumber (CallFunction|MakeUniformString (Variables|Default|GetCurrentIndex) _returnvalue))
  (Rendering|Components|TextRender|SetText (Variables|Default|GetCounter) (Utilities|Text|ToText(String) (Utilities|String|Append _stringnumber "/" (Utilities|String|ToString(Integer) (- _returnvalue 1))))))

(fn ConstructionScript)

(fn GetMax
  (return (Transformation|GetWorldLocation (Variables|Default|Getmax))))

(fn GetMin
  (return (Transformation|GetWorldLocation (Variables|Default|Getmin))))