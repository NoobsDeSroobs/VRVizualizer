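; Data set actor with a Counter component that turns to face the player, likely serving as a readout of the set's data.
; Each Tick calls UpdateData, whose body is not in this graph, then rotates Counter toward player pawn 0 with pitch locked at zero.
; MakeUniformString left-pads a value with zeros to the digit count of the given array size, producing fixed-width number strings.
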(event EventTick
  (params (DeltaSeconds :type Float%20%28single-precision%29))
  (bind _returnvalue (Game|Player|GetPlayerPawn 0))
  (bind _counter (Variables|Default|GetCounter))
  (bind _returnvalue_2 (Transformation|GetActorLocation _returnvalue))
  (bind _returnvalue_3 (Transformation|GetWorldLocation _counter))
  (bind _returnvalue_4 (Math|Rotator|FindLookatRotation _returnvalue_3 _returnvalue_2))
  (bind (_roll _pitch _yaw) (Math|Rotator|BreakRotator _returnvalue_4))
  (Class|Grabbable|UpdateData)
  (Transformation|SetWorldRotation (Variables|Default|GetCounter) (Math|Rotator|MakeRotator _roll 0.0 _yaw) false true))

(fn ConstructionScript)

(fn MakeUniformString
  (params (Value :type Integer) (ArraySize :type Integer))
  (Variables|Default|SetVal Value)
  (bind _output_get (LocalVariables|SetArrSize ArraySize))
  (while (> _output_get 9)
    (Math|Integer|IncrementInt (LocalVariables|GetNumDigits)
      (:%20%20
        (LocalVariables|SetArrSize (/ (LocalVariables|GetArrSize) 10)))))
  (LocalVariables|SetTempVal (Variables|Default|GetVal))
  (while (> (LocalVariables|GetTempVal) 9)
    (Math|Integer|IncrementInt (LocalVariables|GetNumValDigits)
      (:%20%20
        (LocalVariables|SetTempVal (/ (LocalVariables|GetTempVal) 10)))))
  (for _index (range 1 (- (LocalVariables|GetNumDigits) (LocalVariables|GetNumValDigits)))
    (LocalVariables|SetRetStr (Utilities|String|Append (LocalVariables|GetRetStr) "0")))
  (bind _output_get_2 (LocalVariables|SetRetStr (Utilities|String|Append (LocalVariables|GetRetStr) (Utilities|String|ToString(Integer) (Variables|Default|GetVal)))))
  (return _output_get_2))