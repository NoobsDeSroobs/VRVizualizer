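; GeoArteryBP is an actor that animates an artery as a flipbook of 18 static meshes, with a text counter for the current frame.
; BeginPlay or SetupAsSubActor fills the mesh array and derives SwitchTime from LoopTime, also disabling collision and overlaps on the box.
; Tick advances the index through a gate that PlayPause toggles, while Previous and Next step manually.
; UpdateMesh swaps the mesh, applies the vertex-colour material and refreshes the counter.
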(event Custom|UpdateMesh
  (bind _arterymeshes (Variables|Default|GetArteryMeshes))
  (bind _returnvalue (Utilities|Array|Length _arterymeshes))
  ;[1 1 1] UpdateMesh
  (Components|StaticMesh|SetStaticMesh (Variables|Default|GetArtery) (Utilities|Array|Get(acopy) (Variables|Default|GetArteryMeshes) (Variables|Default|GetCurrentIndex)))
  (Rendering|Material|SetMaterial (Variables|Default|GetArtery) 0 "/Game/Materials/VertexColour.VertexColour")
  (Collision|SetCollisionEnabled (Variables|Default|GetArtery) "NoCollision")
  (bind _stringnumber (CallFunction|MakeUniformString (Variables|Default|GetCurrentIndex) _returnvalue))
  (Rendering|Components|TextRender|SetText (Variables|Default|GetCounter) (Utilities|Text|ToText(String) (Utilities|String|Append _stringnumber "/" (Utilities|String|ToString(Integer) (- _returnvalue 1))))))

(event Custom|SetupAsSubActor
  (bind _box (Variables|Default|GetBox))
  (bind _arterymeshes (Variables|Default|GetArteryMeshes))
  (Utilities|Array|Clear (Variables|Default|GetArteryMeshes))
  ;[1 1 1] Init
  (Utilities|Array|Add _arterymeshes "/Game/Chromosome/Artery/StaticMeshes/GeometricMeshes/ArteryGeo0.ArteryGeo0")
  (Utilities|Array|Add _arterymeshes "/Game/Chromosome/Artery/StaticMeshes/GeometricMeshes/ArteryGeo1.ArteryGeo1")
  (Utilities|Array|Add _arterymeshes "/Game/Chromosome/Artery/StaticMeshes/GeometricMeshes/ArteryGeo2.ArteryGeo2")
  (Utilities|Array|Add _arterymeshes "/Game/Chromosome/Artery/StaticMeshes/GeometricMeshes/ArteryGeo3.ArteryGeo3")
  (Utilities|Array|Add _arterymeshes "/Game/Chromosome/Artery/StaticMeshes/GeometricMeshes/ArteryGeo4.ArteryGeo4")
  (Utilities|Array|Add _arterymeshes "/Game/Chromosome/Artery/StaticMeshes/GeometricMeshes/ArteryGeo5.ArteryGeo5")
  (Utilities|Array|Add _arterymeshes "/Game/Chromosome/Artery/StaticMeshes/GeometricMeshes/ArteryGeo6.ArteryGeo6")
  (Utilities|Array|Add _arterymeshes "/Game/Chromosome/Artery/StaticMeshes/GeometricMeshes/ArteryGeo7.ArteryGeo7")
  (Utilities|Array|Add _arterymeshes "/Game/Chromosome/Artery/StaticMeshes/GeometricMeshes/ArteryGeo8.ArteryGeo8")
  (Utilities|Array|Add _arterymeshes "/Game/Chromosome/Artery/StaticMeshes/GeometricMeshes/ArteryGeo9.ArteryGeo9")
  (Utilities|Array|Add _arterymeshes "/Game/Chromosome/Artery/StaticMeshes/GeometricMeshes/ArteryGeo10.ArteryGeo10")
  (Utilities|Array|Add _arterymeshes "/Game/Chromosome/Artery/StaticMeshes/GeometricMeshes/ArteryGeo11.ArteryGeo11")
  (Utilities|Array|Add _arterymeshes "/Game/Chromosome/Artery/StaticMeshes/GeometricMeshes/ArteryGeo12.ArteryGeo12")
  (Utilities|Array|Add _arterymeshes "/Game/Chromosome/Artery/StaticMeshes/GeometricMeshes/ArteryGeo13.ArteryGeo13")
  (Utilities|Array|Add _arterymeshes "/Game/Chromosome/Artery/StaticMeshes/GeometricMeshes/ArteryGeo14.ArteryGeo14")
  (Utilities|Array|Add _arterymeshes "/Game/Chromosome/Artery/StaticMeshes/GeometricMeshes/ArteryGeo15.ArteryGeo15")
  (Utilities|Array|Add _arterymeshes "/Game/Chromosome/Artery/StaticMeshes/GeometricMeshes/ArteryGeo16.ArteryGeo16")
  (Utilities|Array|Add _arterymeshes "/Game/Chromosome/Artery/StaticMeshes/GeometricMeshes/ArteryGeo17.ArteryGeo17")
  (Variables|Default|SetSwitchTime (/ (Variables|Default|GetLoopTime) (Math|Conversions|ToFloat(Integer) (Utilities|Array|Length (Variables|Default|GetArteryMeshes)))))
  (Collision|SetCollisionEnabled _box "NoCollision")
  (Components|Activation|SetActive _box false false)
  (Variables|/Script/Engine.PrimitiveComponent|SetbGenerateOverlapEvents _box false))

(event EventBeginPlay
  (bind _box (Variables|Default|GetBox))
  (bind _arterymeshes (Variables|Default|GetArteryMeshes))
  ;[1 1 1] Init
  (Utilities|Array|Add _arterymeshes "/Game/Chromosome/Artery/StaticMeshes/GeometricMeshes/ArteryGeo0.ArteryGeo0")
  (Utilities|Array|Add _arterymeshes "/Game/Chromosome/Artery/StaticMeshes/GeometricMeshes/ArteryGeo1.ArteryGeo1")
  (Utilities|Array|Add _arterymeshes "/Game/Chromosome/Artery/StaticMeshes/GeometricMeshes/ArteryGeo2.ArteryGeo2")
  (Utilities|Array|Add _arterymeshes "/Game/Chromosome/Artery/StaticMeshes/GeometricMeshes/ArteryGeo3.ArteryGeo3")
  (Utilities|Array|Add _arterymeshes "/Game/Chromosome/Artery/StaticMeshes/GeometricMeshes/ArteryGeo4.ArteryGeo4")
  (Utilities|Array|Add _arterymeshes "/Game/Chromosome/Artery/StaticMeshes/GeometricMeshes/ArteryGeo5.ArteryGeo5")
  (Utilities|Array|Add _arterymeshes "/Game/Chromosome/Artery/StaticMeshes/GeometricMeshes/ArteryGeo6.ArteryGeo6")
  (Utilities|Array|Add _arterymeshes "/Game/Chromosome/Artery/StaticMeshes/GeometricMeshes/ArteryGeo7.ArteryGeo7")
  (Utilities|Array|Add _arterymeshes "/Game/Chromosome/Artery/StaticMeshes/GeometricMeshes/ArteryGeo8.ArteryGeo8")
  (Utilities|Array|Add _arterymeshes "/Game/Chromosome/Artery/StaticMeshes/GeometricMeshes/ArteryGeo9.ArteryGeo9")
  (Utilities|Array|Add _arterymeshes "/Game/Chromosome/Artery/StaticMeshes/GeometricMeshes/ArteryGeo10.ArteryGeo10")
  (Utilities|Array|Add _arterymeshes "/Game/Chromosome/Artery/StaticMeshes/GeometricMeshes/ArteryGeo11.ArteryGeo11")
  (Utilities|Array|Add _arterymeshes "/Game/Chromosome/Artery/StaticMeshes/GeometricMeshes/ArteryGeo12.ArteryGeo12")
  (Utilities|Array|Add _arterymeshes "/Game/Chromosome/Artery/StaticMeshes/GeometricMeshes/ArteryGeo13.ArteryGeo13")
  (Utilities|Array|Add _arterymeshes "/Game/Chromosome/Artery/StaticMeshes/GeometricMeshes/ArteryGeo14.ArteryGeo14")
  (Utilities|Array|Add _arterymeshes "/Game/Chromosome/Artery/StaticMeshes/GeometricMeshes/ArteryGeo15.ArteryGeo15")
  (Utilities|Array|Add _arterymeshes "/Game/Chromosome/Artery/StaticMeshes/GeometricMeshes/ArteryGeo16.ArteryGeo16")
  (Utilities|Array|Add _arterymeshes "/Game/Chromosome/Artery/StaticMeshes/GeometricMeshes/ArteryGeo17.ArteryGeo17")
  (Variables|Default|SetSwitchTime (/ (Variables|Default|GetLoopTime) (Math|Conversions|ToFloat(Integer) (Utilities|Array|Length (Variables|Default|GetArteryMeshes)))))
  (Collision|SetCollisionEnabled _box "NoCollision")
  (Components|Activation|SetActive _box false false)
  (Variables|/Script/Engine.PrimitiveComponent|SetbGenerateOverlapEvents _box false))

(event EventTick
  (params (DeltaSeconds :type Float%20%28single-precision%29))
  (|CallParentFunction DeltaSeconds)
  (Utilities|FlowControl|Gate false
    (:Exit
      (bind _continuekana (CallFunction|Update DeltaSeconds))
      (if _continuekana
        (Variables|Default|SetCurrentIndex (Utilities|Increment (Variables|Default|GetCurrentIndex) (Variables|Default|GetArteryMeshes)))
        (CallFunction|UpdateMesh)))))

(event EventPrevious
  (Variables|Default|SetCurrentIndex (Utilities|Decrement (Variables|Default|GetCurrentIndex) (Variables|Default|GetArteryMeshes)))
  (CallFunction|UpdateMesh))

(event EventNext
  (Variables|Default|SetCurrentIndex (Utilities|Increment (Variables|Default|GetCurrentIndex) (Variables|Default|GetArteryMeshes)))
  (CallFunction|UpdateMesh))

(event EventPlayPause
  (Utilities|FlowControl|Gate false) ; enters at Toggle
)

(fn ConstructionScript)